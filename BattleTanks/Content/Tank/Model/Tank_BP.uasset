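; Player-controllable tank Blueprint that wires input to its aiming and movement components.
; On BeginPlay it passes the barrel and turret to TankAiming and the two tracks to TankMovement.
; Aim axes yaw an azimuth gimbal and pitch the spring arm within a clamped range, orbiting the view independently of the turret.
; Move and turn axes feed TankMovement, while the Fire action calls TankAiming.Fire.
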(event EventBeginPlay
  (Class|TankAimingComponent|Initialise (Variables|Default|GetTankAiming) (Variables|Default|GetBarrel) (Variables|Default|GetTurret))
  (Class|TankMovementComponent|Initialise (Variables|Default|GetTankMovement) (Variables|Default|GetTrack_L) (Variables|Default|GetTrack_R)))

(event Input|ActionEvents|InputActionFire
  (params (Key :type Key%20Structure))
  ;[1 1 1] Fire System
  (:Pressed
    (Class|TankAimingComponent|Fire (Variables|Default|GetTankAiming))))

(event Input|AxisEvents|InputAxisAimAzimuth
  (params (AxisValue :type Float%20%28single-precision%29))
  ;[1 1 1] Barrel-Turret Movement
  (Transformation|AddLocalRotation (Variables|Default|GetAzimuth%20gimbal) (Math|Rotator|MakeRotator 0.0 0.0 AxisValue) false false))

(event Input|AxisEvents|InputAxisMoveForward
  (params (AxisValue :type Float%20%28single-precision%29))
  ;[1 1 1] Tank Movement
  (Class|TankMovementComponent|MoveForward (Variables|Default|GetTankMovement) AxisValue))

(event Input|AxisEvents|InputAxisTurnRight
  (params (AxisValue :type Float%20%28single-precision%29))
  ;[1 1 1] Tank Movement
  (Class|TankMovementComponent|TurnRight (Variables|Default|GetTankMovement) AxisValue))

(event Input|AxisEvents|InputAxisAimElevation
  (params (AxisValue :type Float%20%28single-precision%29))
  ;[1 1 1] Barrel-Turret Movement
  (Transformation|SetRelativeLocationAndRotation (Variables|Default|GetSpringArm) "0, 0, 0" (Math|Rotator|MakeRotator 0.0 (Math|Float|Clamp(Float) (+ AxisValue (.Pitch (Math|Rotator|BreakRotator (Variables|/Script/Engine.SceneComponent|GetRelativeRotation (Variables|Default|GetSpringArm))))) -3e+01 -1e+01) 0.0) false false))

(fn ConstructionScript)